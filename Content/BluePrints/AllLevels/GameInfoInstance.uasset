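; Game instance Blueprint that manages front-end menus and multiplayer sessions.
; A save-game check opens the main menu or, without a save, the options menu; Show events create the widgets, caching all but the server menu.
; Launch and join events show a loading screen, then create a session and open Lobby as listen server, or join one.
; Failures and network or travel errors route to DisplayErrorMessage, which, like both error-string helpers, is an empty stub.
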(event Custom|ShowMainMenu
  (bind _returnvalue (Game|GetPlayerController 0))
  (Utilities|IsValid (Variables|Widgets|GetMainMenu_WB)
    (:Is%20Valid
      _)
    (:Is%20Not%20Valid
      (bind _returnvalue_2 (UserInterface|CreateWidget "/Game/BluePrints/UI/MainMenu/MainMenu.MainMenu_C" _returnvalue))
      (Variables|Widgets|SetMainMenu_WB _returnvalue_2)))
  (UserInterface|Viewport|AddtoViewport (Variables|Widgets|GetMainMenu_WB) 0)
  (Variables|/Script/Engine.PlayerController|SetbShowMouseCursor _returnvalue false))

(event Custom|ShowHostMenu
  (Utilities|IsValid (Variables|Widgets|GetHostMenu_WB)
    (:Is%20Valid
      _)
    (:Is%20Not%20Valid
      (bind _returnvalue (UserInterface|CreateWidget "/Game/BluePrints/UI/MainMenu/HostMenu.HostMenu_C" (Game|GetPlayerController 0)))
      (Variables|Widgets|SetHostMenu_WB _returnvalue)))
  (UserInterface|Viewport|AddtoViewport (Variables|Widgets|GetHostMenu_WB) 0))

(event Custom|ShowServerMenu
  (bind _returnvalue (UserInterface|CreateWidget "/Game/BluePrints/UI/MainMenu/ServerMenu.ServerMenu_C" (Game|GetPlayerController 0)))
  (UserInterface|Viewport|AddtoViewport _returnvalue 0))

(event Custom|ShowOptionsMenu
  (Utilities|IsValid (Variables|Widgets|GetOptionsMenu_WB)
    (:Is%20Valid
      _)
    (:Is%20Not%20Valid
      (bind _returnvalue (UserInterface|CreateWidget "/Game/BluePrints/UI/MainMenu/OptionsMenu.OptionsMenu_C" (Game|GetPlayerController 0)))
      (Variables|Widgets|SetOptionsMenu_WB _returnvalue)))
  (UserInterface|Viewport|AddtoViewport (Variables|Widgets|GetOptionsMenu_WB) 0))

(event Custom|LaunchLobby
  (params (NumberOfPlayers :type Integer) (EnableLan? :type Boolean) (ServerName :type Text))
  (Variables|ServerSettings|SetMaxPlayers NumberOfPlayers)
  (Variables|ServerSettings|SetServerName ServerName)
  (CallFunction|ShowLoadingScreen)
  (|Session (Game|GetPlayerController 0) (Variables|ServerSettings|GetMaxPlayers) EnableLan?
    (:OnSuccess
      (Game|OpenLevel(byName) "Lobby" true "listen"))
    (:OnFailure
      (Utilities|DisplayErrorMessage "Failed to create session, please try again"))))

(event Custom|ShowLoadingScreen
  (Utilities|IsValid (Variables|Widgets|GetLoadingScreen_WB)
    (:Is%20Valid
      _)
    (:Is%20Not%20Valid
      (bind _returnvalue (UserInterface|CreateWidget "/Game/BluePrints/UI/AllLevels/LoadingScreen.LoadingScreen_C" (Game|GetPlayerController 0)))
      (Variables|Widgets|SetLoadingScreen_WB _returnvalue)))
  (UserInterface|Viewport|AddtoViewport (Variables|Widgets|GetLoadingScreen_WB) 0))

(event Custom|JoinServer
  (params (SessionToJoin :type Blueprint%20Session%20Result%20Structure))
  (CallFunction|ShowLoadingScreen)
  (|JoinSession (Game|GetPlayerController 0) SessionToJoin
    (:OnFailure
      (Utilities|DisplayErrorMessage "Failed to join session, please try again"))))

(event Custom|DestroySessionCaller
  (params (PlayerController :type Player%20Controller%20Object%20Reference))
  ;[1 1 1] Destroy session when called
  (|DestroySession PlayerController))

(event Custom|SaveGameCheck
  (bind _returnvalue (SaveGame|DoesSaveGameExist (Variables|Default|GetPlayerSettingsSave)))
  (if _returnvalue
    (CallFunction|ShowMainMenu)
    (Variables|Default|SetCreatedSaveFileCheck true)
    (else
      (CallFunction|ShowOptionsMenu)
      (Variables|/Script/Engine.PlayerController|SetbShowMouseCursor (Game|GetPlayerController 0) true))))

(event EventHandleNetworkError
  (params (FailureType :type ENetworkFailure%20Enum :default "NetDriverAlreadyExists") (bIsServer :type Boolean))
  ;[1 1 1] Handle Network Error, Displays message
  (if bIsServer
    _
    (else
      _))
  (Utilities|DisplayErrorMessage (CallFunction|NetErrorString FailureType)))

(event EventHandleTravelError
  (params (FailureType :type ETravelFailure%20Enum :default "NoLevel"))
  ;[1 1 1] Handles Travel errors and displays message
  (Utilities|DisplayErrorMessage (CallFunction|TravelErrorString FailureType)))

(fn NetErrorString
  (params (FailureType :type ENetworkFailure%20Enum :default "NetDriverAlreadyExists"))
  (return ""))

(fn TravelErrorString
  (params (FailureType :type ETravelFailure%20Enum :default "NoLevel"))
  (return ""))