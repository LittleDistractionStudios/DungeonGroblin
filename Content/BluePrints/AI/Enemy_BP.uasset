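; Enemy AI character that perceives and chases Groblin_BP, punches it, and dies into a ragdoll before being destroyed.
; AI perception writes line of sight and target to the blackboard, clearing them through a timer after sight is lost.
; A toggleable right-fist overlap volume deals damage during the punch montage.
; Health is clamped on hurt and linked to a health bar widget via a character reference.
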(event OnTargetPerceptionUpdated(AIPerception)
  (params (Actor :type Actor%20Object%20Reference) (Stimulus :type AI%20Stimulus%20Structure))
  (bind _returnvalue (AI|GetBlackboard 0))
  (bind _asgroblin_bp (Utilities|Casting|CastToGroblin_BP Actor))
  (if (Utilities|Struct|BreakAIStimulus Stimulus)
    (Utilities|Time|ClearandInvalidateTimerbyHandle (Variables|Default|GetEnemyTimer))
    (AI|Components|Blackboard|SetValueasBool _returnvalue (Variables|Default|GetHasLineOfSight) true)
    (AI|Components|Blackboard|SetValueasObject _returnvalue (Variables|Default|GetEnemyActor) _asgroblin_bp)
    (else
      (bind _returnvalue_2 (Utilities|Time|SetTimerbyEvent (delegate Custom|StartEnemyTimer) (Variables|Default|GetLineOfSightTimer)))
      (Variables|Default|SetEnemyTimer _returnvalue_2))))

(event OnComponentBeginOverlap(RightFistHurtbox)
  (params (OverlappedComponent :type Primitive%20Component%20Object%20Reference) (OtherActor :type Actor%20Object%20Reference) (OtherComp :type Primitive%20Component%20Object%20Reference) (OtherBodyIndex :type Integer) (bFromSweep :type Boolean) (SweepResult :type Hit%20Result%20Structure%20%28by%20ref%29))
  (if (Variables|Combat|GetHurtboxActive)
    (bind _asgroblin_bp (Utilities|Casting|CastToGroblin_BP OtherActor))
    (Default|Hurt _asgroblin_bp 25.0)))

(event Custom|Hurt
  (params (Damage :type Float%20%28single-precision%29))
  (Variables|Stats|SetHealth (Math|Float|Clamp(Float) (- (Variables|Stats|GetHealth) Damage) 0.0 (Variables|Stats|GetMaxHealth)))
  (Variables|Combat|SetIsHurt true)
  (if (== (Variables|Stats|GetHealth) 0.0)
    (Variables|Combat|SetIsDead true)
    (CallFunction|Death)
    (else
      (Variables|Combat|SetIsHurt false))))

(event Custom|Death
  (bind _mesh (Variables|Character|GetMesh))
  (Physics|SetSimulatePhysics _mesh true)
  (Collision|SetCollisionEnabled _mesh "QueryAndPhysics")
  (Utilities|FlowControl|Delay 3.0)
  (Actor|DestroyActor))

(event Custom|Attack
  (bind _returnvalue (Animation|PlayAnimMontage "/Game/Assets/Characters/Enemies/Mushroom_Man/Mushroom_Man_Animations/punching_Montage.Punching_Montage" 1.0 "None"))
  (Variables|Default|SetAnimLength _returnvalue))

(event Custom|StartEnemyTimer
  (bind _returnvalue (AI|GetBlackboard 0))
  (AI|Components|Blackboard|SetValueasBool _returnvalue (Variables|Default|GetHasLineOfSight) false)
  (AI|Components|Blackboard|SetValueasObject _returnvalue (Variables|Default|GetEnemyActor) 0))

(event Custom|HurtboxToggle
  (params (Hurt%20Box%20Active :type Boolean))
  (bind _output_get (Variables|Combat|SetHurtboxActive Hurt%20Box%20Active))
  (Variables|/Script/Engine.PrimitiveComponent|SetbGenerateOverlapEvents (Variables|Default|GetRightFistHurtbox) _output_get))

(event EventBeginPlay
  (bind _asenemy_health_bar (Utilities|Casting|CastToEnemyHealthBar (UserInterface|GetUserWidgetObject (Variables|Default|GetHealthBar))))
  (Variables|/Game/BluePrints/UI/EnemyHealthBar.EnemyHealthBar_C|SetCharacterRef _asenemy_health_bar self))

(fn ConstructionScript)

(fn UpdateWalkSpeed
  (params (NewWalkSpeed :type Float%20%28single-precision%29))
  (Variables|/Script/Engine.CharacterMovementComponent|SetMaxWalkSpeed (Variables|Character|GetCharacterMovement) NewWalkSpeed))