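; NPC Blueprint that plays networked melee punch animations for a mushroom man character.
; MeleeAttackCheck branches on authority, calling the multicast event directly on authority or routing through the server event on remote, which also prints an error message.
; The multicast event uses a FlipFlop to alternate between two punch montages on the mesh.
; MeleeAttack is an empty event, and no damage or hit detection is present.
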(event Custom|MeleeAttackMulticast
  (bind _mesh (Variables|Character|GetMesh))
  (Utilities|FlowControl|FlipFlop
    (:A
      (Animation|Montage|PlayMontage _mesh "/Game/Assets/Characters/Enemies/New_Mushroom_Man/Animations/Mushroom_Man_Anim_Punch_Montage.Mushroom_Man_Anim_Punch_Montage"))
    (:B
      (Animation|Montage|PlayMontage _mesh "/Game/Assets/Characters/Enemies/New_Mushroom_Man/Animations/Mushroom_Man_Anim_PunchMushroom_Montage.Mushroom_Man_Anim_PunchMushroom_Montage"))))

(event Custom|MeleeAttackServer
  (CallFunction|MeleeAttackMulticast))

(event Custom|MeleeAttackCheck
  (Networking|SwitchHasAuthority
    (:Authority
      (CallFunction|MeleeAttackMulticast))
    (:Remote
      (CallFunction|MeleeAttackServer)
      (Development|PrintString "error! meote ran attack"))))

(event EventMeleeAttack)

(fn ConstructionScript)