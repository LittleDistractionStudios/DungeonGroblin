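; Gameplay player controller that handles character spawning, HUD and chat for each player.
; On local BeginPlay it loads saved player settings and passes them to the server, where HacknSlash_GM respawns the player with the chosen character, then HUD setup follows.
; Chat messages relay through the GameMode's controller list to update every player's chat window.
; FlipFlops toggle chat border visibility on T and the mouse cursor through an event.
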(event Custom|PassCharacterInfoToServer
  (params (PlayerSettingsInfo :type Player%20Info%20Structure))
  ;[1 1 1] Passes character info and respawns player with selected character, then calls set up chat window
  (Variables|Default|SetPlayerSettings PlayerSettingsInfo)
  (bind _ashackn_slash_gm (Utilities|Casting|CastToHacknSlash_GM (Game|GetGameMode)))
  (Default|RespawnPlayer _ashackn_slash_gm self (.MyPlayerCharacter (Utilities|Struct|BreakPlayerInfo (Variables|Default|GetPlayerSettings))))
  (CallFunction|SetupHUD))

(event Custom|SetupHUD
  ;[1 1 1] Creates GameplayChat and adds to Viewport
  (Utilities|IsValid (Variables|Default|GetHudWB)
    (:Is%20Valid
      (Viewport|RemoveAllWidgets))
    (:Is%20Not%20Valid
      _))
  (bind _returnvalue (UserInterface|CreateWidget "/Game/BluePrints/UI/AllLevels/HUD.HUD_C"))
  (bind _output_get (Variables|Default|SetHudWB _returnvalue))
  (UserInterface|Viewport|AddtoViewport _output_get 0))

(event Custom|GetChatMessage
  (params (TextToSend :type Text))
  ;[1 1 1] Process and handle incoming chat and calls update on client
  (Variables|Default|SetTextToSend TextToSend)
  (Variables|Default|SetSenderName (.MyPlayerName (Utilities|Struct|BreakPlayerInfo (Variables|Default|GetPlayerSettings))))
  (bind _ashackn_slash_gm (Utilities|Casting|CastToHacknSlash_GM (Game|GetGameMode)))
  (for _array_element (Variables|/Game/BluePrints/GameMode/HacknSlash_GM.HacknSlash_GM_C|GetAllPlayerControllers _ashackn_slash_gm)
    (bind _asgameplay_pc (Utilities|Casting|CastToGameplay_PC _array_element))
    (CallFunction|UpdateChat _asgameplay_pc (Variables|Default|GetSenderName) (Variables|Default|GetTextToSend))))

(event Custom|UpdateChat
  (params (SenderName :type Text) (SenderText :type Text))
  ;[1 1 1] Updates client chat window
  (Default|UpdateChatWindow (Variables|/Game/BluePrints/UI/AllLevels/HUD.HUD_C|GetChatWindow (Variables|Default|GetHudWB)) SenderName SenderText))

(event Custom|ToggleMouseCursor
  (Utilities|FlowControl|FlipFlop
    (:A
      (Variables|Default|SetbShowMouseCursor true))
    (:B
      (Variables|Default|SetbShowMouseCursor false))))

(event EventBeginPlay
  ;[1 1 1] Loads player info and passes to Server side PlayerController
  (if (Pawn|IsLocalController)
    (Viewport|RemoveAllWidgets)
    (CallFunction|LoadGame)
    (CallFunction|PassCharacterInfotoServer (Variables|Default|GetPlayerSettings))))

(event Input|KeyboardEvents|T
  (params (Key :type Key%20Structure :default "None"))
  (bind _hudwb (Variables|Default|GetHudWB))
  (bind _chatwindow (Variables|/Game/BluePrints/UI/AllLevels/HUD.HUD_C|GetChatWindow _hudwb))
  (bind _borderbit (Variables|/Game/BluePrints/UI/AllLevels/ChatWindow.ChatWindow_C|GetBorderBit _chatwindow))
  (:Pressed
    (Utilities|FlowControl|FlipFlop
      (:A
        (Widget|SetVisibility _borderbit "Visible"))
      (:B
        (Widget|SetVisibility _borderbit "Hidden")))))

(fn ConstructionScript)

(fn LoadGame
  (bind _returnvalue (SaveGame|LoadGamefromSlot (Variables|Default|GetPlayerSettingsSave)))
  (bind _asplayer_save_game (Utilities|Casting|CastToPlayerSaveGame _returnvalue))
  (Variables|Default|SetPlayerSettings (Variables|/Game/BluePrints/AllLevels/PlayerSaveGame.PlayerSaveGame_C|GetS_PlayerInfo _asplayer_save_game)))