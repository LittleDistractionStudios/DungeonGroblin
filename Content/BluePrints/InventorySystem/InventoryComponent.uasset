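; Inventory component that stores items in a fixed-size slot array and shows them in a character sheet for the player or an inventory window otherwise.
; Adding tops up partial stacks, recursing on overflow, or creates a stack, trying reserved leading slots chosen by ItemID for equipment before general slots.
; Toggling lazily creates the widgets on the HUD canvas, then switches their visibility.
; A query totals quantities by item class to check for a required amount.
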(event EventBeginPlay
  (CallFunction|PrepareInventory))

(fn ToggleInventory
  (params (IsPlayer? :type Boolean))
  (bind _charactersheetref (Variables|Default|GetCharacterSheetRef))
  (if IsPlayer?
    (Variables|Default|GetCharacterSheetRef
      (:then
        (if (Widget|IsVisible (Variables|Default|GetCharacterSheetRef))
          (Widget|SetVisibility _charactersheetref "Hidden")
          (else
            (Widget|SetVisibility _charactersheetref "Visible")))
        (Default|RefreshSlots _charactersheetref))
      (:else
        (CallFunction|PrepareInventory)
        (CallFunction|ToggleCharacterSheet)
        (Default|RefreshSlots (Variables|Default|GetCharacterSheetRef))))
    (else
      (Variables|Default|GetInventoryWindowRef
        (:then
          (if (Widget|IsVisible (Variables|Default|GetInventoryWindowRef))
            (Widget|SetVisibility (Variables|Default|GetInventoryWindowRef) "Hidden")
            (else
              (Widget|SetVisibility (Variables|Default|GetInventoryWindowRef) "Visible"))))
        (:else
          (CallFunction|PrepareInventory)
          (bind _returnvalue (UserInterface|CreateWidget "/Game/BluePrints/InventorySystem/InventoryUI/InventoryWindow.InventoryWindow_C" 0 self (Variables|Default|GetInventoryName) 7 0))
          (Variables|Default|SetInventoryWindowRef _returnvalue)
          (bind _returnvalue_2 (Class|CanvasPanel|AddChildtoCanvas (Variables|/Game/BluePrints/UI/AllLevels/HUD.HUD_C|GetCanvasPanel_0 (Variables|/Game/BluePrints/GameMode/Gameplay_PC.Gameplay_PC_C|GetHudWB (.AsGameplay%20PC (Utilities|Casting|CastToGameplay_PC (Game|GetPlayerController 0))))) (Variables|Default|GetInventoryWindowRef)))
          (Class|CanvasPanelSlot|SetAutoSize _returnvalue_2 true)
          (Class|CanvasPanelSlot|SetAlignment _returnvalue_2 "(X=-0.100000,Y=0.500000)")
          (Class|CanvasPanelSlot|SetAnchors _returnvalue_2 (Variables|Default|GetAnchors))
          (Class|CanvasPanelSlot|SetPosition _returnvalue_2 (Variables|Default|GetPositions)))))))

(fn AddtoInventory
  (params (ContentToAdd :type Slot%20Structure%20Structure))
  (if (.isstackable (.itemstructure ContentToAdd))
    (bind _slotindex (Utilities|HasPartialStack ContentToAdd)
      (:True
        (bind _success (CallFunction|AddtoStack ContentToAdd _slotindex))
        (LocalVariables|SetIsSuccessful _success)
        (return (LocalVariables|GetIsSuccessful) _slotindex))
      (:False
        (bind (_success_2 _indexnumber) (CallFunction|CreateStack ContentToAdd))
        (LocalVariables|SetIsSuccessful _success_2)
        (return (LocalVariables|GetIsSuccessful) _indexnumber)))
    (else
      (bind (_success_3 _indexnumber_2) (CallFunction|CreateStack (Utilities|Struct|MakeSlotStructure (.itemstructure ContentToAdd) 1)))
      (LocalVariables|SetIsSuccessful _success_3)
      (return (LocalVariables|GetIsSuccessful) _indexnumber_2))))

(fn PrepareInventory
  (Utilities|Array|Resize (Variables|Default|GetInventory) (Variables|Default|GetNumberOfSlots))
  (for (_array_element _array_index) (Variables|Default|GetInventory)
    (if (!= (.Class (Utilities|Struct|BreakItemStructure (.itemstructure _array_element))) 0)
      (Utilities|Array|SetArrayElem (Variables|Default|GetInventory) _array_index (Utilities|Struct|MakeSlotStructure (Utilities|GetClassDefaults (.Class (Utilities|Struct|BreakItemStructure (.itemstructure _array_element)))) (.quantity _array_element)))
      (else
        (Utilities|Array|SetArrayElem (Variables|Default|GetInventory) _array_index (Utilities|Struct|MakeSlotStructure "(ItemID_42_F887A633490D7ED7C53EE89A36FAEAE8=0,Name_3_7ACDF1834A6226A19A96A5835E711453=\"\",ToolTip_28_56735DCD4F7620A850756FBE5570B5C7=NSLOCTEXT(\"[C77113FE49BA80D991FB64A9B802FC98]\", \"F59D3EAE485BA5CF105EA6AA003A1B3B\", \"Default Value\"),IsConsumable_15_89D214A34F0E06DDDDFC108DF5932990=True,IsStackable_6_2B1002484F706B23D1ADADB22060F3A8=True,MaxStackSize_38_032D82144A697A0EB543DA8F20535130=0,ItemImage_12_320D63E64FF6732F769CF5B669928504=None,Class_34_D6514E63436BFCF55D106DA9BB6A82EF=None,Rarity_47_782DBD4F449A05AE2761309BA13453E0=NewEnumerator0,IsEquipment_50_7A77F7CC4DC01D44D6DE2E8B2A736478=False)" 0))))))

(fn CreateStack
  (params (ContentToAdd :type Slot%20Structure%20Structure))
  (bind _itemstructure (Utilities|Struct|BreakSlotStructure ContentToAdd))
  (if (.isequipment _itemstructure)
    (if (== (.itemid _itemstructure) 1)
      (bind (_array_element _array_index) (Utilities|Array|ForEachLoopwithBreak (Variables|Default|GetInventory) :!label _label)
        (:LoopBody
          (if (>= _array_index 2)
            (goto _label Break)
            (elif (<= (.quantity _array_element) 0)
              (LocalVariables|SetHasSpace true)
              (LocalVariables|SetIdentifiedIndex _array_index)
              (goto _label Break)
              (else
                (LocalVariables|SetHasSpace false)))))
        (:Completed
          (if (LocalVariables|GetHasSpace)
            (Utilities|Array|SetArrayElem (Variables|Default|GetInventory) (LocalVariables|GetIdentifiedIndex) ContentToAdd :!label _label_2)
            (return (LocalVariables|GetHasSpace) (LocalVariables|GetIdentifiedIndex))
            (else
              (bind (_array_element_2 _array_index_2) (Utilities|Array|ForEachLoopwithBreak (Variables|Default|GetInventory) :!label _label_3)
                (:LoopBody
                  (if (>= _array_index_2 6)
                    (if (<= (.quantity _array_element_2) 0)
                      (LocalVariables|SetHasSpace true)
                      (LocalVariables|SetIdentifiedIndex _array_index_2)
                      (goto _label_3 Break)
                      (else
                        (LocalVariables|SetHasSpace false)))))
                (:Completed
                  (if (LocalVariables|GetHasSpace)
                    (Utilities|Array|SetArrayElem (Variables|Default|GetInventory) (LocalVariables|GetIdentifiedIndex) ContentToAdd)
                    (return (LocalVariables|GetHasSpace) (LocalVariables|GetIdentifiedIndex))
                    (else
                      (return false 0)))))))))
      (elif (<= (.Quantity (Utilities|Struct|BreakSlotStructure (Utilities|Array|Get(acopy) (Variables|Default|GetInventory) (.itemid _itemstructure)))) 0)
        (LocalVariables|SetHasSpace true)
        (LocalVariables|SetIdentifiedIndex (.itemid _itemstructure))
        (goto _label_2)
        (else
          (LocalVariables|SetHasSpace false)
          (goto _label_3))))
    (else
      (goto _label_3))))

(fn AddtoStack
  (params (SlotStructure :type Slot%20Structure%20Structure) (SlotIndex :type Integer))
  (bind _inventory (Variables|Default|GetInventory))
  (bind _inventory_2 (Variables|Default|GetInventory))
  (bind _maxstacksize (Utilities|Struct|BreakItemStructure (.itemstructure SlotStructure)))
  (bind _output (Utilities|Array|Get(acopy) _inventory_2 SlotIndex))
  (bind _output_2 (Utilities|Array|Get(acopy) _inventory SlotIndex))
  (bind _output_get (LocalVariables|SetCurrentQuantity (.quantity _output_2)))
  (if (> (+ _output_get (.Quantity (Utilities|Struct|BreakSlotStructure SlotStructure))) (.maxstacksize (.itemstructure _output_2)))
    (Utilities|Array|SetArrayElem (Variables|Default|GetInventory) SlotIndex (Utilities|Struct|MakeSlotStructure (.itemstructure SlotStructure) _maxstacksize))
    (CallFunction|AddtoInventory (Utilities|Struct|MakeSlotStructure (.itemstructure SlotStructure) (- (.quantity SlotStructure) (- _maxstacksize (LocalVariables|GetCurrentQuantity)))))
    (else
      (Utilities|Array|SetArrayElem _inventory_2 SlotIndex (Utilities|Struct|MakeSlotStructure (.itemstructure _output) (+ (.quantity _output) (.quantity SlotStructure))))))
  (return true))

(fn InventoryQuery
  (params (QueryItem :type Item%20Class%20Reference) (QueryQuantity :type Integer))
  (bind _array_element (Utilities|Array|ForEachLoopwithBreak (Variables|Default|GetInventory))
    (:LoopBody
      (if (== (.Class (Utilities|Struct|BreakItemStructure (.itemstructure _array_element))) QueryItem)
        (LocalVariables|SetRunningTotal (+ (LocalVariables|GetRunningTotal) (.quantity _array_element)))))
    (:Completed
      (return (>= (LocalVariables|GetRunningTotal) QueryQuantity)))))

(fn ToggleCharacterSheet
  (bind _returnvalue (UserInterface|CreateWidget "/Game/BluePrints/InventorySystem/InventoryUI/CharacterSheet.CharacterSheet_C" 0 self 0 5))
  (Variables|Default|SetCharacterSheetRef _returnvalue)
  (bind _returnvalue_2 (Class|CanvasPanel|AddChildtoCanvas (Variables|/Game/BluePrints/UI/AllLevels/HUD.HUD_C|GetCanvasPanel_0 (Variables|/Game/BluePrints/GameMode/Gameplay_PC.Gameplay_PC_C|GetHudWB (.AsGameplay%20PC (Utilities|Casting|CastToGameplay_PC (Game|GetPlayerController 0))))) (Variables|Default|GetCharacterSheetRef)))
  (Class|CanvasPanelSlot|SetAutoSize _returnvalue_2 true)
  (Class|CanvasPanelSlot|SetAlignment _returnvalue_2 "(X=1.100000,Y=0.500000)")
  (Class|CanvasPanelSlot|SetAnchors _returnvalue_2 (Variables|Default|GetAnchors))
  (Class|CanvasPanelSlot|SetPosition _returnvalue_2 (Variables|Default|GetPositions)))